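; Test actor for a FroxComputeFlow component that feeds it a float frame and displays the computed output in the world.
; On BeginPlay it fills a square frame with the Value variable and sets it as the InTest input.
; Each Tick runs the flow and writes the first element of the OutTest frame to a TextRender.
; The bound value-changed handler checks for OutTest but takes no action.
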(event `self.ReceiveBeginPlay`
  (add `FroxComputeFlowComponent.OnValueChanged` (`self.FroxComputeFlow`) (delegate `OnValueChanged`))
  ;[1 1 1] Create Frame
  (bind _returnvalue (`FroxBlueprintLibrary.MakeFrame` 64 64))
  (`FroxComputeFrame.FillFloat` _returnvalue (`self.Value`))
  (`FroxComputeFlowComponent.SetValueAsFrame` (`self.FroxComputeFlow`) (`self.InTest`) _returnvalue))

(event `OnValueChanged`
  (params (Name :type Name))
  ;[1 1 1] Read Out Value
  (if (== Name (`self.OutTest`))
    _))

(event `self.ReceiveTick`
  (params (DeltaSeconds :type "Float (single-precision)"))
  (`FroxComputeFlowComponent.Perform` (`self.FroxComputeFlow`))
  ;[1 1 1] Read Out Value
  (`TextRenderComponent.K2_SetText` (`self.TextRender`) (`KismetTextLibrary.Conv_DoubleToText` (`FroxComputeFrame.AtFloat` (`FroxComputeFlowComponent.GetValueAsFrame` (`self.FroxComputeFlow`) (`self.OutTest`)) 0 0) "HalfToEven")))

(fn `UserConstructionScript`)