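; BP_Flip is an actor that feeds vertical and horizontal flags into a HeightMapFlow and shows its height map on a dynamic grid mesh, apparently to demonstrate flipping.
; On BeginPlay it binds to the flow's value-changed event, then sets both booleans by key name.
; When the height map key changes, it pulls that frame from the flow and applies it to the mesh, with no Tick logic.
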(event `self.ReceiveBeginPlay`
  (bind _heightmapflow (`self.HeightMapFlow`))
  (add `FroxComputeFlowComponent.OnValueChanged` (`self.HeightMapFlow`) (delegate `OnFlowChanged`))
  (`FroxComputeFlowComponent.SetValueAsBool` _heightmapflow (`self.VerticalName`) (`self.Vertical`))
  (`FroxComputeFlowComponent.SetValueAsBool` _heightmapflow (`self.HorizontalName`) (`self.Horizontal`)))

(event `OnFlowChanged`
  (params (Name :type Name))
  (bind _heightmapname (`self.HeightMapName`))
  (if (== Name _heightmapname)
    (`DyanmicGridMeshComponent.SetHeightMap` (`self.DyanmicGridMesh`) (`FroxComputeFlowComponent.GetValueAsFrame` (`self.HeightMapFlow`) _heightmapname))))

(fn `UserConstructionScript`)